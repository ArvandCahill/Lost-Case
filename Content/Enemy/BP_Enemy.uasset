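; Horror-game enemy that uses PawnSensing to chase a seen player or investigate noises with AIMoveTo.
; Sightings raise move speed and alter game speed/FOV settings; a retriggerable delay ends the chase when sightings stop.
; Noises within hearing range are weighted by distance, and loudness sets approach speed unless chasing.
; RandomRoam is empty with its navmesh wandering logic disconnected, and the overlap jumpscare only prints a debug string.
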(event OnHearNoise(PawnSensing)
  (params (Instigator :type Pawn%20Object%20Reference) (Location :type Vector%20%28by%20ref%29 :default "0, 0, 0") (Volume :type Float%20%28single-precision%29))
  (bind _returnvalue (Transformation|GetActorLocation))
  (bind _returnvalue_2 (Math|Vector|Distance(Vector) Location _returnvalue))
  (bind _returnvalue_3 (/ _returnvalue_2 3e+03))
  (bind _returnvalue_4 (Math|Float|Lerp 1.0 0.0 _returnvalue_3))
  (bind _returnvalue_5 (* Volume _returnvalue_4))
  ;[1 1 1] Go To Noise
  (bind _output_get (Variables|Default|SethearingRange (Variables|/Script/AIModule.PawnSensingComponent|GetHearingThreshold (Variables|Default|GetPawnSensing))))
  (if (<= _returnvalue_2 _output_get)
    (Development|PrintString (Utilities|String|ToString(Float) _returnvalue_5))
    (if (> _returnvalue_5 0.25)
      (if (not (Variables|Default|GetisChasing))
        (Variables|Default|SetisHearing true)
        (Variables|/Script/Engine.CharacterMovementComponent|SetMaxWalkSpeed (Variables|Character|GetCharacterMovement) (* Volume 1e+03))
        (AI|AIMoveTo self Location 0 1e+02 false
          (:then
            (Utilities|FlowControl|RetriggerableDelay 2.0)
            (CallFunction|RandomRoam))
          (:OnSuccess
            (Variables|Default|SetisHearing false)))))))

(event OnComponentBeginOverlap(SphereCollision)
  (params (OverlappedComponent :type Primitive%20Component%20Object%20Reference) (OtherActor :type Actor%20Object%20Reference) (OtherComp :type Primitive%20Component%20Object%20Reference) (OtherBodyIndex :type Integer) (bFromSweep :type Boolean) (SweepResult :type Hit%20Result%20Structure%20%28by%20ref%29))
  ;[1 1 1] Trigger Jumpscare
  (Utilities|Casting|CastToHorrorEngineCharacter OtherActor)
  (if true
    (Development|PrintString "Khumskare")))

(event OnSeePawn(PawnSensing)
  (params (Pawn :type Pawn%20Object%20Reference))
  ;[1 1 1] Chasing
  (Utilities|Casting|CastToHorrorEngineCharacter Pawn)
  (CallFunction|ChangeGameSettings 1e+02 5e+02 1e+03 32.0 1.2e+02 8e+01)
  (Variables|/Script/Engine.CharacterMovementComponent|SetMaxWalkSpeed (Variables|Character|GetCharacterMovement) 1e+03)
  (Variables|Default|SetisChasing true)
  (AI|AIMoveTo self "0, 0, 0" Pawn 1e+02 false
    (:then
      (Utilities|FlowControl|RetriggerableDelay 1.0)
      (Variables|Default|SetisChasing false)
      (CallFunction|ChangeGameSettings 1e+02 1.5e+02 3e+02 32.0 9e+01 6e+01)
      (CallFunction|RandomRoam))))

(event Custom|Random%20Roam
  ;[1 1 1] Random Roam
)

(event EventBeginPlay
  ;[1 1 1] Begin Play
  (CallFunction|RandomRoam))

(fn ConstructionScript)