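; Settings helper library that saves, loads and applies the game's player preferences through a SaveBP_Settings save slot.
; Load creates a default save when none exists, then returns the stored struct.
; Inject re-reads it per value, pushing display, scalability, frame limit and VSync through GameUserSettings, and gamma and FSR3/frame generation through console commands.
; Outside MenuLevel it also sets the player's look sensitivity and HorrorEngineCharacter voice detection options.
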(fn SaveSettingsPreferences
  (params (SettingsPreferences :type Struct%20Settings%20Structure))
  (bind _returnvalue (SaveGame|CreateSaveGameObject "/Game/Blueprint/BlueprintDataManager/SaveBP_Settings.SaveBP_Settings_C"))
  (Variables|/Game/Blueprint/BlueprintDataManager/SaveBP_Settings.SaveBP_Settings_C|SetSettingsPreferences _returnvalue SettingsPreferences)
  (SaveGame|SaveGametoSlot _returnvalue (LocalVariables|GetSlot%20Name)))

(fn LoadSettingsPreferences
  (bind _returnvalue (SaveGame|DoesSaveGameExist (LocalVariables|GetSlot%20Name)))
  (if _returnvalue
    _
    (else
      (CallFunction|SaveSettingsPreferences (Utilities|Struct|MakeStruct_Settings "Fullscreen" "NewEnumerator2" false))))
  (bind _returnvalue_2 (SaveGame|LoadGamefromSlot (LocalVariables|GetSlot%20Name)))
  (bind _assave_bp_settings (Utilities|Casting|CastToSaveBP_Settings _returnvalue_2))
  (return (Variables|/Game/Blueprint/BlueprintDataManager/SaveBP_Settings.SaveBP_Settings_C|GetSettingsPreferences _assave_bp_settings)))

(fn InjectSettingPreference
  (bind _settings_preferences (CallFunction|LoadSettingsPreferences))
  (bind _returnvalue (Utilities|String|EnumtoString (.fps _settings_preferences)))
  (bind _returnvalue_2 (Settings|GetGameUserSettings))
  (Class|GameUserSettings|SetFullscreenMode _returnvalue_2 (.windowmode _settings_preferences))
  (Class|GameUserSettings|SetScreenResolution _returnvalue_2 (Utilities|Select :Index (.windowresolution _settings_preferences) :NewEnumerator0 (Utilities|Struct|MakeIntPoint 1280 720) :NewEnumerator1 (Utilities|Struct|MakeIntPoint 1600 900) :NewEnumerator2 (Utilities|Struct|MakeIntPoint 1920 1080) :NewEnumerator3 (Utilities|Struct|MakeIntPoint 2560 1440) :NewEnumerator4 (Utilities|Struct|MakeIntPoint 3840 2160)))
  (Development|PrintString 0 "Kentir")
  (Development|ExecuteConsoleCommand 0 (Utilities|String|ToString(Text) (Utilities|Text|FormatText "r.gamma {value}" (Math|Float|Lerp 1.0 3.0 (.brightness _settings_preferences)))) 0)
  (Class|GameUserSettings|SetOverallScalabilityLevel _returnvalue_2 (+ (Math|Conversions|ToInteger(Byte) (.graphics _settings_preferences)) 1))
  (Development|ExecuteConsoleCommand 0 (Utilities|String|ToString(Text) (Utilities|Text|FormatText "r.FidelityFX.FSR3.QualityMode {Value}" (Math|Conversions|ToInteger(Byte) (.fsr _settings_preferences)))) 0)
  (Development|ExecuteConsoleCommand 0 (Utilities|String|ToString(Text) (Utilities|Text|FormatText "r.FidelityFX.FI.Enabled {Value}" (Math|Integer|SelectInt 1 0 (.framegeneration _settings_preferences)))) 0)
  (Class|GameUserSettings|SetFrameRateLimit _returnvalue_2 (Math|Conversions|ToFloat(Integer) (Math|Integer|SelectInt 999 (Math|Conversions|ToInteger(Byte) _returnvalue) (Utilities|Enum|Equal(Enum) _returnvalue "Unlimited"))))
  (Class|GameUserSettings|SetVSyncEnabled _returnvalue_2 (.vsync _settings_preferences))
  (Utilities|FlowControl|Sequence
    (:then_1
      (bind _returnvalue_3 (Game|GetCurrentLevelName 0))
      (if (not (Utilities|Enum|Equal(Enum) _returnvalue_3 "MenuLevel"))
        (bind _asmaster (CallFunction|GetPlayer))
        (Variables|/Game/HorrorEngine/HorrorEngine.HorrorEngine_C|SetLookSensivity _asmaster (Math|Float|Lerp 0.1 2.0 (.camerasensivity _settings_preferences)))
        (bind _ashorror_engine_character (Utilities|Casting|CastToHorrorEngineCharacter (Game|GetPlayerCharacter 0)))
        (Variables|/Game/HorrorEngine/Blueprints/Core/HorrorEngineCharacter.HorrorEngineCharacter_C|SetVoiceDetectionEnable _ashorror_engine_character (.voicedetection _settings_preferences))
        (Variables|/Game/HorrorEngine/Blueprints/Core/HorrorEngineCharacter.HorrorEngineCharacter_C|SetVoiceSensivity _ashorror_engine_character (.voicesensivity _settings_preferences))))))