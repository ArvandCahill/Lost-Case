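; Horror Engine base character that handles movement input, footstep and landing head shake, and movement noise for pawn noise sensing.
; Forward and strafe axes add movement input and trigger the player's head shake, with strafing disabled while flying.
; Tick emits noise scaled by running, walking or crouching, though its threshold tests only the forward axis, twice.
; Landing triggers a separate head shake and full-loudness noise.
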(event EventTick
  (params (DeltaSeconds :type Float%20%28single-precision%29))
  ;[0.498 0.6745 1] Movement Noise
  (if (or (or (> (Variables|Movement|GetMovementAxisVerticalValue) (Variables|Movement|GetNoiseValueTolerant)) (< (Variables|Movement|GetMovementAxisVerticalValue) (* (Variables|Movement|GetNoiseValueTolerant) -1.0))) (or (> (Variables|Movement|GetMovementAxisVerticalValue) (Variables|Movement|GetNoiseValueTolerant)) (< (Variables|Movement|GetMovementAxisVerticalValue) (* (Variables|Movement|GetNoiseValueTolerant) -1.0))))
    (bind _asmaster (CallFunction|GetPlayer))
    (if (Variables|/Game/HorrorEngine/HorrorEngine.HorrorEngine_C|GetRunning _asmaster)
      (Variables|Movement|SetNoiseValue 1.0)
      (elif (Variables|/Game/HorrorEngine/HorrorEngine.HorrorEngine_C|GetCrouching _asmaster)
        (Variables|Movement|SetNoiseValue 0.0)
        (else
          (Variables|Movement|SetNoiseValue 0.25))))
    (Class|PawnNoiseEmitterComponent|MakeNoise (Variables|Default|GetPawnNoiseEmitter) self (Variables|Movement|GetNoiseValue) (Transformation|GetActorLocation))))

(event EventOnLanded
  (params (Hit :type Hit%20Result%20Structure%20%28by%20ref%29))
  ;[0.498 0.6737 1] Jump Settings
  (bind _asmaster (CallFunction|GetPlayer))
  (Default|Footstep/Headshake _asmaster "NewEnumerator1")
  (Class|PawnNoiseEmitterComponent|MakeNoise (Variables|Default|GetPawnNoiseEmitter) self 1.0 (Transformation|GetActorLocation)))

(event Input|AxisEvents|InputAxis[HE]MoveForward
  (params (AxisValue :type Float%20%28single-precision%29))
  ;[0.498 0.6745 1] Movement
  (Variables|Movement|SetMovementAxisVerticalValue AxisValue)
  (Pawn|Input|AddMovementInput (Math|Vector|GetForwardVector (Transformation|GetActorRotation)) AxisValue false)
  (bind _asmaster (CallFunction|GetPlayer))
  (Default|Footstep/Headshake _asmaster "NewEnumerator0"))

(event Input|AxisEvents|InputAxis[HE]MoveRight
  (params (AxisValue :type Float%20%28single-precision%29))
  ;[0.498 0.6745 1] Movement
  (Variables|Movement|SetMovementAxisHorizontalValue AxisValue)
  (if (not (Class|NavMovementComponent|IsFlying (Variables|Character|GetCharacterMovement)))
    (Pawn|Input|AddMovementInput (Math|Vector|GetRightVector (Transformation|GetActorRotation)) AxisValue false)
    (bind _asmaster (CallFunction|GetPlayer))
    (Default|Footstep/Headshake _asmaster "NewEnumerator0")))

(fn ConstructionScript)