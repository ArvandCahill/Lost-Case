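; BP_fog is a trigger volume that changes the level's exponential height fog density as the player enters or leaves it, apparently a home area.
; Sphere overlap begin and end each wait about ten seconds, then check for the Player tag and find the ExponentialHeightFog actor.
; Separate in-home and out-home timelines then play from the start, driving that fog's density on each update.
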(event OnComponentBeginOverlap(Sphere)
  (params (OverlappedComponent :type Primitive%20Component%20Object%20Reference) (OtherActor :type Actor%20Object%20Reference) (OtherComp :type Primitive%20Component%20Object%20Reference) (OtherBodyIndex :type Integer) (bFromSweep :type Boolean) (SweepResult :type Hit%20Result%20Structure%20%28by%20ref%29))
  (Utilities|FlowControl|Delay 10.1)
  (if (Actor|ActorHasTag OtherActor "Player")
    (bind _returnvalue (Actor|GetActorOfClass "/Script/Engine.ExponentialHeightFog"))
    (bind _fogdensityinhome (Timeline|FogDensityInHome PlayFromStart)
      (:Update
        (Class|ExponentialHeightFogComponent|SetFogDensity (Variables|/Script/Engine.ExponentialHeightFog|GetComponent _returnvalue) _fogdensityinhome)))))

(event OnComponentEndOverlap(Sphere)
  (params (OverlappedComponent :type Primitive%20Component%20Object%20Reference) (OtherActor :type Actor%20Object%20Reference) (OtherComp :type Primitive%20Component%20Object%20Reference) (OtherBodyIndex :type Integer))
  (Utilities|FlowControl|Delay 10.1)
  (if (Actor|ActorHasTag OtherActor "Player")
    (bind _returnvalue (Actor|GetActorOfClass "/Script/Engine.ExponentialHeightFog"))
    (bind _fogdensityouthome (Timeline|FogDensityOutHome PlayFromStart)
      (:Update
        (Class|ExponentialHeightFogComponent|SetFogDensity (Variables|/Script/Engine.ExponentialHeightFog|GetComponent _returnvalue) _fogdensityouthome)))))

(fn ConstructionScript)